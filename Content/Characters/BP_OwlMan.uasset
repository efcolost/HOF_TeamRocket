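; BP_OwlMan is a hostile character that respawns the player on contact and can be knocked into physics by a thrown rock.
; While IsStunned is false, its OverlapCollision sends an overlapping BP_Player to Respawn, or switches the mesh to simulated physics when hit by BP_ThrowableRock.
; The graph never sets IsStunned, so a rock hit leaves the respawn check active.
; The ApproachingSound overlap only casts to the player and does nothing further.
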(event `self.ReceiveBeginPlay`
  (`PrimitiveComponent.SetSimulatePhysics` (`self.Mesh`) false))

(event `self.OverlapCollision.OnComponentBeginOverlap`
  (params (OverlappedComponent :type "PrimitiveComponent Object Reference") (OtherActor :type "Actor Object Reference") (OtherComp :type "PrimitiveComponent Object Reference") (OtherBodyIndex :type Integer) (bFromSweep :type Boolean) (SweepResult :type "HitResult Structure (by ref)"))
  (bind _mesh (`self.Mesh`))
  ;[1 1 1] Overlaps with player
  ;;[1 1 1] self not stunned
  (if (not (`self.IsStunned?`))
    (cast `/Game/Blueprints/BP_ThrowableRock` OtherActor
      (:`then`
        (`PrimitiveComponent.SetSimulatePhysics` (`self.Mesh`) true)
        (`PrimitiveComponent.SetCollisionObjectType` _mesh "ECC_PhysicsBody")
        (`PrimitiveComponent.SetCollisionEnabled` _mesh "QueryAndPhysics"))
      (:`CastFailed`
        (bind _asbp_player (cast `/Game/Player/BP_Player` OtherActor))
        (`/Game/Player/BP_Player.Respawn` _asbp_player)))))

(event `self.ApproachingSound.OnComponentBeginOverlap`
  (params (OverlappedComponent :type "PrimitiveComponent Object Reference") (OtherActor :type "Actor Object Reference") (OtherComp :type "PrimitiveComponent Object Reference") (OtherBodyIndex :type Integer) (bFromSweep :type Boolean) (SweepResult :type "HitResult Structure (by ref)"))
  (cast `/Game/Player/BP_Player` OtherActor))

(fn `UserConstructionScript`)