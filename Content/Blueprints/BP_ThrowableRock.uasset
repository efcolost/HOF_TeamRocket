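; BP_ThrowableRock is a rock actor that stays free of gravity until it is thrown.
; On BeginPlay it zeroes its projectile movement speeds, disables gravity on its sphere and binds ThrowRock to a RockThrown event.
; When thrown, the sphere starts simulating physics, gets a velocity-change impulse along its forward vector scaled by Strength, applied at the Scene component's location, then re-enables gravity.
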(event `self.ReceiveBeginPlay`
  (bind _projectilemovement (`self.ProjectileMovement`))
  (set `ProjectileMovementComponent.MaxSpeed` 0.0 _projectilemovement)
  (set `ProjectileMovementComponent.InitialSpeed` 0.0 _projectilemovement)
  (`PrimitiveComponent.SetEnableGravity` (`self.Sphere`) false)
  (add `self.RockThrown` (delegate `ThrowRock`)))

(event `ThrowRock`
  (bind _sphere (`self.Sphere`))
  (`PrimitiveComponent.SetSimulatePhysics` _sphere true)
  (`PrimitiveComponent.AddVelocityChangeImpulseAtLocation` _sphere (* (`SceneComponent.GetForwardVector` _sphere) (`self.Strength`)) (`SceneComponent.K2_GetComponentLocation` (`self.Scene`)) "None")
  (`PrimitiveComponent.SetEnableGravity` _sphere true))

(fn `UserConstructionScript`)