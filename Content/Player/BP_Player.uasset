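; Player character with Enhanced Input movement, look and sprint, plus picking up and throwing rocks.
; Capsule overlaps track a nearby BP_Rock, which Interact destroys and replaces with a spawned BP_ThrowableRock.
; Tick pins the held rock to ItemLocation with capsule rotation until Interact throws it, before any new pickup in that press.
; Respawn reloads M_Level1.
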(event `self.ReceiveBeginPlay`
  ;[0 1 0.3693 1 130] Movement
  (bind _asplayer_controller (cast `PlayerController` (`self.GetController`)))
  (bind _returnvalue (pcsubsystem `EnhancedInputLocalPlayerSubsystem` _asplayer_controller))
  (`/Engine/EditorBlueprintResources/StandardMacros.IsValid` _returnvalue
    (:`Is Valid`
      (`EnhancedInputSubsystemInterface.AddMappingContext` _returnvalue "/Game/Controllers/Input/IMC_InputMappings.IMC_InputMappings" 0 (struct)))))

(event `EnhancedInput|/Game/Controllers/Input/IA_Move`
  (params (ActionValue :type "Vector2D Structure") (ElapsedSeconds :type "Float (double-precision)") (TriggeredSeconds :type "Float (double-precision)") (InputAction :type "InputAction Object Reference" :default "/Game/Controllers/Input/IA_Move.IA_Move"))
  (bind (_returnvalue_roll _returnvalue_pitch _returnvalue_yaw) (`KismetMathLibrary.BreakRotator` (`self.GetControlRotation`)))
  (bind (_returnvalue_roll_2 _returnvalue_pitch_2 _returnvalue_yaw_2) (`KismetMathLibrary.BreakRotator` (`self.GetControlRotation`)))
  ;[0 1 0.3693 1 130] Movement
  (:`Triggered`
    (`self.AddMovementInput` (`KismetMathLibrary.GetRightVector` (`KismetMathLibrary.MakeRotator` _returnvalue_roll 0.0 _returnvalue_yaw)) ActionValue_X)
    (`self.AddMovementInput` (`KismetMathLibrary.GetForwardVector` (`KismetMathLibrary.MakeRotator` 0.0 0.0 _returnvalue_yaw_2)) ActionValue_Y)))

(event `EnhancedInput|/Game/Controllers/Input/IA_Look`
  (params (ActionValue :type "Vector2D Structure") (ElapsedSeconds :type "Float (double-precision)") (TriggeredSeconds :type "Float (double-precision)") (InputAction :type "InputAction Object Reference" :default "/Game/Controllers/Input/IA_Look.IA_Look"))
  ;[0 1 0.3693 1 130] Movement
  (:`Triggered`
    (`self.AddControllerYawInput` ActionValue_X)
    (bind _result (`/Engine/EditorBlueprintResources/StandardMacros.NegateFloat` ActionValue_Y)
      (:`  `
        (`self.AddControllerPitchInput` _result)))))

(event `EnhancedInput|/Game/Controllers/Input/IA_Sprint`
  (params (ActionValue :type Boolean) (ElapsedSeconds :type "Float (double-precision)") (TriggeredSeconds :type "Float (double-precision)") (InputAction :type "InputAction Object Reference" :default "/Game/Controllers/Input/IA_Sprint.IA_Sprint"))
  ;[0 1 0.3693 1 130] Movement
  (:`Triggered`
    (set `self.IsSprinting?` true)
    (set `CharacterMovementComponent.MaxWalkSpeed` 900.0 (`self.CharacterMovement`)))
  (:`Completed`
    (set `self.IsSprinting?` false)
    (set `CharacterMovementComponent.MaxWalkSpeed` 600.0 (`self.CharacterMovement`))))

(event `self.ReceiveTick`
  (params (DeltaSeconds :type "Float (single-precision)"))
  (bind _throwablerock (`self.ThrowableRock`))
  (bind _sphere (`/Game/Blueprints/BP_ThrowableRock.Sphere` _throwablerock))
  (if (`self.HoldingRock?`)
    (`/Engine/EditorBlueprintResources/StandardMacros.IsValid` _throwablerock
      (:`Is Valid`
        (`SceneComponent.K2_SetWorldLocation` _sphere (`SceneComponent.K2_GetComponentLocation` (`self.ItemLocation`)) false false)
        (`SceneComponent.K2_SetWorldRotation` _sphere (`SceneComponent.K2_GetComponentRotation` (`self.CapsuleComponent`)) false false)))))

(event `self.CapsuleComponent.OnComponentBeginOverlap`
  (params (OverlappedComponent :type "PrimitiveComponent Object Reference") (OtherActor :type "Actor Object Reference") (OtherComp :type "PrimitiveComponent Object Reference") (OtherBodyIndex :type Integer) (bFromSweep :type Boolean) (SweepResult :type "HitResult Structure (by ref)"))
  (bind _asbp_rock (cast `/Game/Blueprints/BP_Rock` OtherActor))
  (set `self.OverlappingRock` true)
  (set `self.OverlappedRock` _asbp_rock))

(event `self.CapsuleComponent.OnComponentEndOverlap`
  (params (OverlappedComponent :type "PrimitiveComponent Object Reference") (OtherActor :type "Actor Object Reference") (OtherComp :type "PrimitiveComponent Object Reference") (OtherBodyIndex :type Integer))
  (cast `/Game/Blueprints/BP_Rock` OtherActor)
  (set `self.OverlappingRock` false)
  (set `self.OverlappedRock` null))

(event `EnhancedInput|/Game/Controllers/Input/IA_Interact`
  (params (ActionValue :type Boolean) (ElapsedSeconds :type "Float (double-precision)") (TriggeredSeconds :type "Float (double-precision)") (InputAction :type "InputAction Object Reference" :default "/Game/Controllers/Input/IA_Interact.IA_Interact"))
  (:`Triggered`
    (`KismetSystemLibrary.PrintString` "Triggered")
    (`|ExecutionSequence`
      (:`then_0`
        (if (`self.HoldingRock?`)
          (`self.ThrowItem`)))
      (:`then_1`
        (if (`self.OverlappingRock`)
          (`self.K2_DestroyActor` (`self.OverlappedRock`))
          (`self.PickUpItem`)
          (`KismetSystemLibrary.PrintString` "Picked up Item"))))))

(fn `PickUpItem`
  (bind _returnvalue (`|SpawnActorFromClass` "/Game/Blueprints/BP_ThrowableRock.BP_ThrowableRock_C" (`SceneComponent.K2_GetComponentToWorld` (`self.ItemLocation`)) "Undefined" "MultiplyWithRoot" null null))
  (set `self.ThrowableRock` _returnvalue)
  (set `self.HoldingRock?` true)
  (set `self.RockThrown?` false))

(fn `Respawn`
  (`GameplayStatics.OpenLevel` "M_Level1"))

(fn `ThrowItem`
  (set `self.RockThrown?` true)
  (set `self.HoldingRock?` false)
  (`/Game/Blueprints/BP_ThrowableRock.RockThrown` (`self.ThrowableRock`))
  (`KismetSystemLibrary.PrintString` "Called"))

(fn `UserConstructionScript`)