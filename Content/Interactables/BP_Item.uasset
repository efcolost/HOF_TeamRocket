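; BP_Item is a pickup interactable with a "to pick up" prompt that destroys itself when interacted with.
; Interact prints an "Added to the inventory" message, plays a click sound at its location and removes the actor, without storing any inventory data.
; Getters expose interaction type, hold duration, tap count and widget styling, and an event sets the remaining required taps.
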(event `/Game/InteractionSystem/BPI_Interactable.Interact`
  (params (Interactor :type "Actor Object Reference"))
  (`KismetSystemLibrary.PrintString` (`KismetTextLibrary.Conv_TextToString` (`|FormatText` "Added {ItemName} to the inventory of {ActorName}" (`KismetSystemLibrary.GetDisplayName` self) Interactor)))
  (`GameplayStatics.PlaySoundAtLocation` "/Engine/VREditor/Sounds/VR_click3.VR_click3" (`self.K2_GetActorLocation`) (struct) 1.0 1.0 0.0 null null null null)
  (`self.K2_DestroyActor`))

(event `self.SetRequiredTapsRemaining`
  (params (RequiredTapsCounter :type Integer))
  (set `self.RequiredTapsCounter` RequiredTapsCounter))

(fn `GetHoldDuration`
  (returns (Duration :type "Float (double-precision)"))
  (return (`self.HoldDuration`)))

(fn `GetInteractionLocation`
  (returns (Location :type "Vector Structure"))
  (return (0.0 0.0 0.0)))

(fn `GetInteractionPrompt`
  (returns (Value :type Text))
  (return "to pick up"))

(fn `GetInteractionType`
  (returns (Type :type "/Game/InteractionSystem/E_InteractionTypes Enum"))
  (return (`self.InteractionType`)))

(fn `GetTotalTaps`
  (returns (TotalTaps :type Integer))
  (return (`self.TotalTaps`)))

(fn `GetWidgetBackgroundColor`
  (returns (Color :type "SlateColor Structure"))
  (return (`self.BackgroundBarColor`)))

(fn `GetWidgetBlurStrength`
  (returns (BlurStrength :type "Float (double-precision)"))
  (return (`self.BlurStrength`)))

(fn `GetWidgetProgressBarColor`
  (returns (Color :type "LinearColor Structure"))
  (return (`self.ProgressBarColor`)))

(fn `UserConstructionScript`)