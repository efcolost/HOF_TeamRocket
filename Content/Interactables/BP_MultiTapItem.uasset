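; Multi-tap pickup item that responds to an Interact event with a "To Pick Up" prompt.
; Interact prints an "added to inventory" message, plays a click sound and destroys the actor, with no inventory write.
; Getters expose interaction type, total taps and widget styling, while hold duration and location return zero.
; The remaining-tap counter resets on BeginPlay and is updated through a setter, with no tap counting here.
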(event `self.ReceiveBeginPlay`
  (set `self.RequiredTapsCounter` 0))

(event `/Game/InteractionSystem/BPI_Interactable.Interact`
  (params (Interactor :type "Actor Object Reference"))
  (`KismetSystemLibrary.PrintString` (`KismetTextLibrary.Conv_TextToString` (`|FormatText` "Added {ItemName} to the inventory of {ActorName}" (`KismetSystemLibrary.GetDisplayName` self) (`KismetSystemLibrary.GetDisplayName` Interactor))))
  (`GameplayStatics.PlaySoundAtLocation` "/Engine/VREditor/Sounds/VR_click3.VR_click3" (`self.K2_GetActorLocation`) (struct) 1.0 1.0 0.0 null null null null)
  (`self.K2_DestroyActor`))

(event `self.SetRequiredTapsRemaining`
  (params (RequiredTapsCounter :type Integer))
  (set `self.RequiredTapsCounter` RequiredTapsCounter))

(fn `GetHoldDuration`
  (returns (Duration :type "Float (double-precision)"))
  (return 0.0))

(fn `GetInteractionLocation`
  (returns (Location :type "Vector Structure"))
  (return (0.0 0.0 0.0)))

(fn `GetInteractionPrompt`
  (returns (Value :type Text))
  (return "To Pick Up"))

(fn `GetInteractionType`
  (returns (Type :type "/Game/InteractionSystem/E_InteractionTypes Enum"))
  (return (`self.InteractionType`)))

(fn `GetTotalTaps`
  (returns (TotalTaps :type Integer))
  (return (`self.TotalTaps`)))

(fn `GetWidgetBackgroundColor`
  (returns (Color :type "SlateColor Structure"))
  (return (`self.WidgetBackgroundColor`)))

(fn `GetWidgetBlurStrength`
  (returns (BlurStrength :type "Float (double-precision)"))
  (return (`self.WidgetBlurStrength`)))

(fn `GetWidgetProgressBarColor`
  (returns (Color :type "LinearColor Structure"))
  (return (`self.WidgetProgressBarColor`)))

(fn `UserConstructionScript`)