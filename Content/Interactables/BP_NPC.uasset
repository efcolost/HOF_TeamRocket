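; BP_NPC is an interactable NPC actor that shows a "To talk" prompt.
; On Interact it turns to face the interactor on yaw and plays an item-drop sound at its location; no dialogue logic follows.
; Getter functions supply the interaction system with type, world location, hold and tap requirements, and widget styling from its variables and InteractionLocation component.
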(event `/Game/InteractionSystem/BPI_Interactable.Interact`
  (params (Interactor :type "Actor Object Reference"))
  (bind _returnvalue (`self.K2_GetActorLocation`))
  (bind (_returnvalue_roll _returnvalue_pitch _returnvalue_yaw) (`KismetMathLibrary.BreakRotator` (`KismetMathLibrary.FindLookAtRotation` _returnvalue (`self.K2_GetActorLocation` Interactor))))
  (`self.K2_SetActorRotation` (`KismetMathLibrary.MakeRotator` 0.0 0.0 _returnvalue_yaw))
  (`GameplayStatics.PlaySoundAtLocation` "/Engine/VREditor/Sounds/UI/Drop_Item_From_ContentBrowser.Drop_Item_From_ContentBrowser" _returnvalue (struct) 1.0 1.0 0.0 null null null null))

(fn `GetHoldDuration`
  (returns (Duration :type "Float (double-precision)"))
  (return (`self.HoldDuration`)))

(fn `GetInteractionLocation`
  (returns (Location :type "Vector Structure"))
  (return (`SceneComponent.K2_GetComponentLocation` (`self.InteractionLocation`))))

(fn `GetInteractionPrompt`
  (returns (Value :type Text))
  (return "To talk"))

(fn `GetInteractionType`
  (returns (Type :type "/Game/InteractionSystem/E_InteractionTypes Enum"))
  (return (`self.InteractionType`)))

(fn `GetTotalTaps`
  (returns (TotalTaps :type Integer))
  (return (`self.TotalTaps`)))

(fn `GetWidgetBackgroundColor`
  (returns (Color :type "SlateColor Structure"))
  (return (`self.BackgroundColor`)))

(fn `GetWidgetBlurStrength`
  (returns (BlurStrength :type "Float (double-precision)"))
  (return (`self.BlurStrength`)))

(fn `GetWidgetProgressBarColor`
  (returns (Color :type "LinearColor Structure"))
  (return (`self.ProgressBarColor`)))

(fn `UserConstructionScript`)