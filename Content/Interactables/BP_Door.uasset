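; Interactable door actor that toggles between open and closed when its Interact event fires.
; A timeline drives the door's relative yaw, playing forward to open and reversing to close, with a sound at the door's location when it finishes.
; Getter functions supply the interaction system with location, type, hold and tap settings, widget styling, and a prompt that changes with the open state.
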(event `OpenDoor`
  (set `self.IsOpen?` true)
  (bind (_direction _alpha) (`Timeline|TL_OpenDoor` :!label _label)
    (:`Update`
      (`SceneComponent.K2_SetRelativeRotation` (`self.Door`) (`KismetMathLibrary.MakeRotator` 0.0 0.0 _alpha) false false))
    (:`Finished`
      (`GameplayStatics.PlaySoundAtLocation` "/Engine/VREditor/Sounds/UI/Dockable_Window_Pick_Up.Dockable_Window_Pick_Up" (`SceneComponent.K2_GetComponentLocation` (`self.Door`)) (struct) 1.0 1.0 0.0 null null null null))))

(event `CloseDoor`
  (set `self.IsOpen?` false)
  (goto _label :!via `Reverse`))

(event `/Game/InteractionSystem/BPI_Interactable.Interact`
  (params (Interactor :type "Actor Object Reference"))
  (if (`self.IsOpen?`)
    (`self.CloseDoor`)
    (else
      (`self.OpenDoor`))))

(fn `GetHoldDuration`
  (returns (Duration :type "Float (double-precision)"))
  (return (`self.HoldDuration`)))

(fn `GetInteractionLocation`
  (returns (Location :type "Vector Structure"))
  (return (`SceneComponent.K2_GetComponentLocation` (`self.InteractionLocation`))))

(fn `GetInteractionPrompt`
  (returns (Value :type Text))
  (return (select `bool` (`self.IsOpen?`) :`false` "To open the door" :`true` "To close the door" :!type "Text")))

(fn `GetInteractionType`
  (returns (Type :type "/Game/InteractionSystem/E_InteractionTypes Enum"))
  (return (`self.InteractionType`)))

(fn `GetTotalTaps`
  (returns (TotalTaps :type Integer))
  (return (`self.TotalTaps`)))

(fn `GetWidgetBackgroundColor`
  (returns (Color :type "SlateColor Structure"))
  (return (`self.BackgroundColor`)))

(fn `GetWidgetBlurStrength`
  (returns (BlurStrength :type "Float (double-precision)"))
  (return (`self.BlurStrength`)))

(fn `GetWidgetProgressBarColor`
  (returns (Color :type "LinearColor Structure"))
  (return (`self.ProgressBarColor`)))

(fn `UserConstructionScript`)